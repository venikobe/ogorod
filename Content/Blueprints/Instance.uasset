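; Game instance Blueprint that holds state and shared events for level loading, character skins and score.
; LoadLevel plays a sound, shows an animated loading screen, then opens the named level after a short delay.
; Four Skin events each set a pair of skin and bikini material variables, and AddScoreEvent adds to a running score.
; Several disconnected leftover nodes for sound, HUD and input never run.
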(event `LoadLevel`
  (params (LevelName :type Name))
  (`FMODBlueprintStatics.PlayEvent2D` (`self.LoadingEventSound`))
  (bind _returnvalue (`|CreateWidget` "/Game/Wigets/LoadingScreen/LoadingScreen.LoadingScreen_C"))
  (`UserWidget.AddToViewport` _returnvalue 0)
  (`/Game/Wigets/LoadingScreen/LoadingScreen.Appear` _returnvalue)
  (`KismetSystemLibrary.Delay` 0.6)
  (`GameplayStatics.OpenLevel` LevelName))

(event `Skin1`
  (set `self.MaterialBikini` "/Game/Materials/towel/skin1/Bikini_1.Bikini_1")
  (set `self.MaterialSkin` "/Game/Materials/towel/skin1/RediskaSkin1.RediskaSkin1"))

(event `Skin2`
  (set `self.MaterialBikini` "/Game/Materials/towel/skin2/skindress3.skindress3")
  (set `self.MaterialSkin` "/Game/Materials/towel/skin2/M_Rediska_1_Inst.M_Rediska_1_Inst"))

(event `Skin3`
  (set `self.MaterialBikini` "/Game/Materials/towel/skin3/T_towel2_Mat.T_towel2_Mat")
  (set `self.MaterialSkin` "/Game/Materials/towel/skin3/M_Rediska_2.M_Rediska_2"))

(event `Skin4`
  (set `self.MaterialBikini` "/Game/Materials/towel/skin4/skin4_Mat.skin4_Mat")
  (set `self.MaterialSkin` "/Game/Materials/towel/skin4/M_Rediska_black.M_Rediska_black"))

(event `Add Score Event`
  (params (`To Add` :type Integer))
  (set `self.TheScore` (+ `To Add` (`self.TheScore`))))