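; Actor Blueprint that shows a timed loading screen at BeginPlay, then opens the follow-up UI.
; It hides the cursor, disables player input, adds a LoadingScreen widget and tells it to disappear using TimeToLoad.
; After that time plus a short buffer, OpenUI re-enables input and adds the game mode's HP widget.
; Otherwise OpenShop creates the Shop widget, leaving input disabled here.
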(event `self.ReceiveBeginPlay`
  (bind _returnvalue (`GameplayStatics.GetPlayerController` 0))
  (bind _time_to_load (`self.Time to Load`))
  (`WidgetBlueprintLibrary.SetInputMode_GameOnly` _returnvalue)
  (set `PlayerController.bShowMouseCursor` false _returnvalue)
  (`self.DisableInput` (`GameplayStatics.GetPlayerController` 0) (`GameplayStatics.GetPlayerController` 0))
  (bind _returnvalue_2 (`|CreateWidget` "/Game/Wigets/LoadingScreen/LoadingScreen.LoadingScreen_C"))
  (`UserWidget.AddToViewport` _returnvalue_2 0)
  (`/Game/Wigets/LoadingScreen/LoadingScreen.Disappear` _returnvalue_2 _time_to_load)
  (`KismetSystemLibrary.Delay` (+ _time_to_load 0.35))
  (if (`self.Open UI?`)
    (`self.EnableInput` (`GameplayStatics.GetPlayerController` 0) (`GameplayStatics.GetPlayerController` 0))
    (bind _asbp_third_person_game_mode (cast `/Game/ThirdPerson/Blueprints/BP_ThirdPersonGameMode` (`GameplayStatics.GetGameMode`)))
    (`UserWidget.AddToViewport` (`/Game/ThirdPerson/Blueprints/BP_ThirdPersonGameMode.HpwidhetRef` _asbp_third_person_game_mode) 0)
    (elif (`self.Open Shop?`)
      (bind _returnvalue_3 (`|CreateWidget` "/Game/Wigets/Menu/Shop.Shop_C"))
      (`UserWidget.AddToViewport` _returnvalue_3 0))))

(fn `UserConstructionScript`)