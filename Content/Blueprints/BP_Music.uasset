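; BP_Music is a music manager actor that binds to BP_Speewner's music-start event and plays a starting track.
; When a track finishes, a transition sting plays, then a FlipFlop alternates between two continuing tracks, each looping back through the transition.
; Break and new-wave events swap to and from a rest track.
; The break binding to the spawner is disconnected, so it never runs.
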(event `self.ReceiveBeginPlay`
  (bind _returnvalue (`GameplayStatics.GetActorOfClass` "/Game/AI/Enemies/Spawn/BP_Speewner.BP_Speewner_C"))
  (bind _output_get (set `self.Speewner_ref` _returnvalue))
  (add `/Game/AI/Enemies/Spawn/BP_Speewner.On Music Start` _output_get (delegate `On Music Start_Event`)))

(event `On Music Start_Event`
  (bind _returnvalue (`GameplayStatics.CreateSound2D` (`self.Starting_sound`) 1.0 1.0 0.0 null))
  (set `self.Current_Audio` _returnvalue)
  (`AudioComponent.Play` _returnvalue 0.0)
  (add `AudioComponent.OnAudioFinished` _returnvalue (delegate `Transition`)))

(event `Transition`
  (bind _returnvalue (`GameplayStatics.CreateSound2D` "/Game/Sounds/OST/next_slash.next_slash" 1.0 1.0 0.0 null))
  (set `self.Current_Audio` _returnvalue)
  (`AudioComponent.Play` _returnvalue 0.0)
  (`KismetSystemLibrary.Delay` 1.0)
  (`/Engine/EditorBlueprintResources/StandardMacros.FlipFlop`
    (:`A`
      (`self.Continue_1`))
    (:`B`
      (`self.Continue_2`))))

(event `Continue_1`
  (bind _returnvalue (`GameplayStatics.CreateSound2D` (`self.Continuing1_sound`) 1.0 1.0 0.0 null))
  (set `self.Current_Audio` _returnvalue)
  (`AudioComponent.Play` _returnvalue 0.0)
  (add `AudioComponent.OnAudioFinished` _returnvalue (delegate `Transition`)))

(event `Continue_2`
  (bind _returnvalue (`GameplayStatics.CreateSound2D` (`self.Continuing2_sound`) 1.0 1.0 0.0 null))
  (set `self.Current_Audio` _returnvalue)
  (`AudioComponent.Play` _returnvalue 0.0)
  (add `AudioComponent.OnAudioFinished` _returnvalue (delegate `Transition`)))

(event `On Music Break_Event`
  (`AudioComponent.Stop` (`self.Current_Audio`))
  (bind _returnvalue (`GameplayStatics.CreateSound2D` "/Game/Sounds/OST/rest_slash.rest_slash" 1.0 1.0 0.0 null))
  (`AudioComponent.Play` _returnvalue 0.0))

(event `NewWave`
  (`AudioComponent.Stop` (stale `On Music Break_Event` _returnvalue))
  (`GameplayStatics.PlaySound2D` "/Game/Sounds/OST/transition_slash.transition_slash" 1.0 1.0 0.0 null null)
  (`KismetSystemLibrary.Delay` 3.3)
  (`/Engine/EditorBlueprintResources/StandardMacros.FlipFlop`
    (:`A`
      (`self.Continue_1`))
    (:`B`
      (`self.Continue_2`))))

(fn `UserConstructionScript`)