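; BP_Minion is an AI minion that turns into an enemy when one stays near it too long.
; On BeginPlay an alarm countdown runs, then sends it to a random navigable point near TargetActor.
; Tick polls EnemyNear, stopping AI logic and running a delayed kill countdown with a timeline-driven material color change.
; At zero it increments the game mode's per-level death count, spawns BP_EnemyParent in its place and destroys itself.
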(event `self.ReceiveTick`
  (params (DeltaSeconds :type "Float (single-precision)"))
  (`self.ChinChopa`))

(event `Work`
  (`KismetSystemLibrary.PrintString` "Роботою(пока нет анимации)"))

(event `self.ReceiveBeginPlay`
  (bind _asbp_third_person_game_mode (cast `/Game/ThirdPerson/Blueprints/BP_ThirdPersonGameMode` (`GameplayStatics.GetGameMode`)))
  (set `self.As BP Third Person Game Mode` _asbp_third_person_game_mode)
  (bind _returnvalue (`PrimitiveComponent.CreateDynamicMaterialInstance` (`self.Mesh`) 0 "/Game/AI/Minions/carrot/Materials/carrottexture_Mat.carrottexture_Mat" "None"))
  (set `self.MatInst` _returnvalue)
  (`self.Alarm`))

(event `ChinChopa`
  (bind _as_bp_third_person_game_mode (`self.As BP Third Person Game Mode`))
  (bind _enemynear (`self.EnemyNear`))
  (bind _miniondeathcount (`/Game/ThirdPerson/Blueprints/BP_ThirdPersonGameMode.MinionDeathCount` _as_bp_third_person_game_mode))
  (bind _level_index (`/Game/ThirdPerson/Blueprints/BP_ThirdPersonGameMode.Level Index` _as_bp_third_person_game_mode))
  (if _enemynear
    (`BrainComponent.StopLogic` (`AIController.BrainComponent` (`AIBlueprintHelperLibrary.GetAIController` self)) "")
    (`KismetSystemLibrary.PrintString` (`KismetStringLibrary.Concat_StrStr` "бубийство" (`KismetStringLibrary.Conv_IntToString` (`self.Counter`))) true true (struct :`G` 0.66 :`B` 1.0 :`A` 1.0) 1.0 :!label _label)
    (`self.Colorchange`)
    (if (== (`self.Counter`) 0)
      (`KismetArrayLibrary.Array_Set` _miniondeathcount _level_index (+ (`|GetArrayItem` _miniondeathcount _level_index) 1))
      (`SceneComponent.SetVisibility` (`self.Mesh`) false false)
      (`|SpawnActorFromClass` "/Game/AI/Enemies/BP_EnemyParent.BP_EnemyParent_C" (`KismetMathLibrary.MakeTransform` (`self.K2_GetActorLocation`)) "Undefined" "OverrideRootScale" null null)
      (`self.K2_DestroyActor`)
      (elif _enemynear
        (`KismetSystemLibrary.Delay` 1.0)
        (`/Engine/EditorBlueprintResources/StandardMacros.DecrementInt` (`self.Counter`)
          (:`  `
            (goto _label)))
        (else
          (set `self.Counter` 5))))))

(event `Colorchange`
  (bind (_direction _color) (`Timeline|ColorChangeTimeline`)
    (:`Update`
      (`MaterialInstanceDynamic.SetVectorParameterValue` (`self.MatInst`) "Color" _color))))

(event `Alarm`
  (`KismetSystemLibrary.PrintString` (`KismetStringLibrary.Concat_StrStr` "Тревога через:" (`KismetStringLibrary.Conv_IntToString` (`self.AlarmCounter`))) :!label _label_2)
  (if (== (`self.AlarmCounter`) 0)
    (bind _returnvalue (`GameplayStatics.GetActorOfClass` "/Script/NavigationSystem.RecastNavMesh"))
    (bind _randomlocation (`NavigationSystemV1.K2_GetRandomLocationInNavigableRadius` (`self.K2_GetActorLocation` (`self.Target Actor`)) 100.0 _returnvalue null))
    (`|AIMoveTo` (`PawnMovementComponent.GetPawnOwner` (`self.CharacterMovement`)) _randomlocation null 3.0)
    (else
      (`KismetSystemLibrary.Delay` 1.0)
      (`/Engine/EditorBlueprintResources/StandardMacros.DecrementInt` (`self.AlarmCounter`)
        (:`  `
          (goto _label_2))))))

(fn `UserConstructionScript`)