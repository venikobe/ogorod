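; AI controller for enemies that runs the BH_Enemy behavior tree on BeginPlay.
; Every tick it sets the InAttackRange blackboard key from the distance between the player character and its controlled pawn, using a short fixed threshold.
; Its perception update event is empty, and the logic that would store a perceived BP_Minion in the Minion key is disconnected and never runs.
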(event `self.ReceiveTick`
  (params (DeltaSeconds :type "Float (single-precision)"))
  (`BlackboardComponent.SetValueAsBool` (`AIBlueprintHelperLibrary.GetBlackboard` null) "InAttackRange" (< (`self.GetDistanceTo` (`GameplayStatics.GetPlayerCharacter` 0) (`self.K2_GetPawn`)) 125.0)))

(event `self.ReceiveBeginPlay`
  (`self.RunBehaviorTree` "/Game/AI/Enemies/AI/BH_Enemy.BH_Enemy"))

(event `self.AIPerception.OnTargetPerceptionUpdated`
  (params (Actor :type "Actor Object Reference") (Stimulus :type "AIStimulus Structure")))

(fn `UserConstructionScript`)