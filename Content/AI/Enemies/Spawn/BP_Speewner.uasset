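; Wave-based zombie spawner actor that starts after a printed countdown and spawns random-sized enemy batches with a spawn visual.
; Each enemy gets a random walk speed and is counted and tracked in the game mode.
; When the count reaches the wave's total, it advances the wave after a pause, firing music break/continue calls.
; Otherwise a countdown timer triggers the next batch, and enemies are bound back to the spawn event.
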(event `self.ReceiveBeginPlay`
  ;[0 1 0 0.502] Старт лвла
  (`|ExecutionSequence`
    (:`then_0`
      (set `self.Counter` (`self.InitialCountdown`))
      (`KismetSystemLibrary.PrintString` (`KismetStringLibrary.Concat_StrStr` "Волна через:" (`KismetStringLibrary.Conv_IntToString` (`self.Counter`))) :!label _label)
      (if (== (`self.Counter`) 0)
        (`self.SpawnNextEnemies`)
        (`self.On Music Start`)
        (else
          (`KismetSystemLibrary.Delay` 1.0)
          (`/Engine/EditorBlueprintResources/StandardMacros.DecrementInt` (`self.Counter`)
            (:`  `
              (goto _label))))))
    (:`then_1`
      (bind _asbp_third_person_game_mode (cast `/Game/ThirdPerson/Blueprints/BP_ThirdPersonGameMode` (`GameplayStatics.GetGameMode`)))
      (set `self.As BP Third Person Game Mode` _asbp_third_person_game_mode))))

(event `SpawnTimer`
  (bind _as_bp_third_person_game_mode (`self.As BP Third Person Game Mode`))
  (if (<= (`/Game/ThirdPerson/Blueprints/BP_ThirdPersonGameMode.EnemiesCounter` _as_bp_third_person_game_mode) (`|GetArrayItem` (`/Game/ThirdPerson/Blueprints/BP_ThirdPersonGameMode.EnemiesSum` _as_bp_third_person_game_mode) (`self.WaveCount`)))
    (set `self.Counter` (`self.DelayBetweenEnemies`))
    (`KismetSystemLibrary.PrintString` (`KismetStringLibrary.Concat_StrStr` "Зомби через:" (`KismetStringLibrary.Conv_IntToString` (`self.Counter`))) :!label _label_2)
    (if (== (`self.Counter`) 0)
      (`self.SpawnNextEnemies`)
      (else
        (`KismetSystemLibrary.Delay` 1.0)
        (`/Engine/EditorBlueprintResources/StandardMacros.DecrementInt` (`self.Counter`)
          (:`  `
            (goto _label_2)))))))

(event `SpawnNextEnemies`
  (bind _as_bp_third_person_game_mode (`self.As BP Third Person Game Mode`))
  ;[0 1 0 0.502] Спаун противников
  (`|SpawnActorFromClass` "/Game/AI/Enemies/Spawn/BP_VisualOfSpawning.BP_VisualOfSpawning_C" (`KismetMathLibrary.MakeTransform` (- (`self.K2_GetActorLocation`) (0.0 0.0 20.0))) "Undefined" "OverrideRootScale" null null)
  (`KismetSystemLibrary.Delay` 0.8)
  (for _ (range 1 (+ (`KismetMathLibrary.RandomIntegerInRange` 1 (`|GetArrayItem` (`self.EnemyNum`) (`self.WaveCount`))) 1))
    (`/Engine/EditorBlueprintResources/StandardMacros.IncrementInt` (`/Game/ThirdPerson/Blueprints/BP_ThirdPersonGameMode.EnemiesCounter` (`self.As BP Third Person Game Mode`))
      (:`  `
        (bind _returnvalue (`|SpawnActorFromClass` "/Game/AI/Enemies/BP_EnemyParent.BP_EnemyParent_C" (`KismetMathLibrary.MakeTransform` (`SceneComponent.K2_GetComponentLocation` (`self.EnemiesLocation`)) (`KismetMathLibrary.MakeRotator` 0.0 0.0 (`KismetMathLibrary.RandomFloatInRange` 0.0 180.0))) "Undefined" "OverrideRootScale" null null))
        (`self.Init` _returnvalue)
        (`KismetArrayLibrary.Array_Add` (`/Game/ThirdPerson/Blueprints/BP_ThirdPersonGameMode.Current Enemies Ref` (`self.As BP Third Person Game Mode`)) _returnvalue)
        (if (== (`KismetArrayLibrary.Array_LastIndex` (`self.EnemyNum`)) (`self.WaveCount`))
          (`KismetSystemLibrary.PrintString` "Последняя волна пройдена")
          (elif (>= (`/Game/ThirdPerson/Blueprints/BP_ThirdPersonGameMode.EnemiesCounter` _as_bp_third_person_game_mode) (`|GetArrayItem` (`/Game/ThirdPerson/Blueprints/BP_ThirdPersonGameMode.EnemiesSum` _as_bp_third_person_game_mode) (`self.WaveCount`)))
            (`self.On Music Break`)
            (`/Engine/EditorBlueprintResources/StandardMacros.IncrementInt` (`self.WaveCount`)
              (:`  `
                (`KismetSystemLibrary.Delay` (`KismetMathLibrary.Conv_IntToDouble` (`/Game/ThirdPerson/Blueprints/BP_ThirdPersonGameMode.DelayBetweenWaves` _as_bp_third_person_game_mode)))
                (`self.SpawnNextEnemies`)
                (`KismetSystemLibrary.PrintString` "Новая волна")
                (`self.On Music Continue`)))
            (else
              (`self.SpawnTimer`)
              (`/Engine/EditorBlueprintResources/StandardMacros.IsValid` _returnvalue
                (:`Is Valid`
                  (add `/Game/AI/Enemies/BP_EnemyParent.SpawnNextEnemies` _returnvalue (delegate `SpawnNextEnemies`)))))))))))

(event `BindOnkilled`)

(fn `Init`
  (params (Enemy :type "/Game/AI/Enemies/BP_EnemyParent Object Reference"))
  (`/Engine/EditorBlueprintResources/StandardMacros.IsValid` Enemy
    (:`Is Valid`
      (set `/Game/AI/Enemies/BP_EnemyParent.DelayBetweenEnemies` (`KismetMathLibrary.Conv_IntToDouble` (`self.DelayBetweenEnemies`)) Enemy)
      (bind _output_get (set `CharacterMovementComponent.MaxWalkSpeed` (`KismetMathLibrary.RandomFloatInRange` (`self.SpeedMin`) (`self.SpeedMax`)) (`Character.CharacterMovement` Enemy)))
      (set `/Game/AI/Enemies/BP_EnemyParent.SpeedAtSpawn` _output_get Enemy))))

(fn `UserConstructionScript`)