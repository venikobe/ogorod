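; Enemy spawner trigger that requests a group of enemies when the ShinbiPlayerCharacter enters its Box.
; The first valid overlap disables the Box's collision, then calls RequestSpawn with the group size, billboard location and spawn radius.
; A separate SpawnEnemy event spawns BP_EnemyParent copies at the actor's transform, but its binding to the game mode's RespawnEnemy dispatcher never runs.
; EnemyType is unused.
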(event OnComponentBeginOverlap(Box)
  (params (OverlappedComponent :type Primitive%20Component%20Object%20Reference) (OtherActor :type Actor%20Object%20Reference) (OtherComp :type Primitive%20Component%20Object%20Reference) (OtherBodyIndex :type Integer) (bFromSweep :type Boolean) (SweepResult :type Hit%20Result%20Structure%20%28by%20ref%29))
  (Utilities|Casting|CastToShinbiPlayerCharacter OtherActor)
  (Collision|SetCollisionEnabled (Variables|Default|GetBox) "NoCollision")
  (Default|CallRequestSpawn (Variables|Default|GetSizeOfSpawn) (Transformation|GetWorldLocation (Variables|Default|GetBillboard self)) (Variables|Default|GetRadiusOfSpawn)))

(event Custom|SpawnEnemy
  (for _index (range 0 (- (Variables|Default|GetEnemySpawned) 1))
    (Game|SpawnActorfromClass "/Game/AI/Enemies/BP_EnemyParent.BP_EnemyParent_C" (Transformation|GetActorTransform) "Undefined" 0 0)))

(event EventBeginPlay)

(fn ConstructionScript)