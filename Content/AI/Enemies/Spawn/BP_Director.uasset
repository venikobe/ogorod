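; BP_Director is an AI director that tracks live enemies and fulfils spawn requests from enemy spawners under a MaxEnemies cap.
; At BeginPlay it registers all existing BP_EnemyParent and BP_EnemySpawner actors, binding to their kill and spawn-request events.
; Each request spawns enemies at random reachable navmesh points around the requested location, registering each new one.
; Killed enemies leave the list, and Tick prints the current enemy count for debugging.
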(event `self.ReceiveBeginPlay`
  (`|ExecutionSequence`
    (:`then_0`
      (bind _outactors (`GameplayStatics.GetAllActorsOfClass` "/Game/AI/Enemies/BP_EnemyParent.BP_EnemyParent_C"))
      (for _array_element _outactors
        (`self.OnEnemySpawned` _array_element)))
    (:`then_1`
      (bind _outactors_2 (`GameplayStatics.GetAllActorsOfClass` "/Game/AI/Enemies/Spawn/BP_EnemySpawner.BP_EnemySpawner_C"))
      (for _array_element_2 _outactors_2
        (`self.OnEnemySpawnerSpawned` _array_element_2)))))

(event `self.ReceiveTick`
  (params (DeltaSeconds :type "Float (single-precision)"))
  (`KismetSystemLibrary.PrintString` (`KismetStringLibrary.Concat_StrStr` "Enemies:" (`KismetStringLibrary.Conv_IntToString` (`KismetArrayLibrary.Array_Length` (`self.Enemy`)))) true true (struct :`G` 0.66 :`B` 1.0 :`A` 1.0) 0.0))

(fn `OnEnemyKilled`
  (params (Enemy :type "/Game/AI/Enemies/BP_EnemyParent Object Reference"))
  (`KismetArrayLibrary.Array_RemoveItem` (`self.Enemy`) Enemy))

(fn `OnEnemySpawned`
  (params (Enemy :type "/Game/AI/Enemies/BP_EnemyParent Object Reference"))
  (`KismetArrayLibrary.Array_Add` (`self.Enemy`) Enemy)
  (add `/Game/AI/Enemies/BP_EnemyParent.OnKilled` Enemy (`|CreateDelegate` :!event `OnEnemyKilled`)))

(fn `OnEnemySpawnerSpawned`
  (params (EnemySpawner :type "/Game/AI/Enemies/Spawn/BP_EnemySpawner Object Reference"))
  (`KismetArrayLibrary.Array_Add` (`self.Enemy Spawner`) EnemySpawner)
  (add `/Game/AI/Enemies/Spawn/BP_EnemySpawner.RequestSpawn` EnemySpawner (`|CreateDelegate` :!event `OnEnemySpawnRequested`)))

(fn `OnEnemySpawnRequested`
  (params (Count :type Integer) (Location :type "Vector Structure") (RadiusOfSpawn :type "Float (double-precision)"))
  (for _ (range 1 (+ (`KismetMathLibrary.Min` (- (`self.MaxEnemies`) (`KismetArrayLibrary.Array_Length` (`self.Enemy`))) Count) 1))
    (bind _returnvalue (`|SpawnActorFromClass` "/Game/AI/Enemies/BP_EnemyParent.BP_EnemyParent_C" (`KismetMathLibrary.MakeTransform` (+ (`NavigationSystemV1.K2_GetRandomReachablePointInRadius` Location RadiusOfSpawn null null) (0.0 0.0 88.0))) "Undefined" "OverrideRootScale" null null))
    (`/Engine/EditorBlueprintResources/StandardMacros.IsValid` _returnvalue
      (:`Is Valid`
        (`self.OnEnemySpawned` _returnvalue)))))

(fn `UserConstructionScript`)